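; Base rifle weapon actor, meant to be a child actor of a pawn, that fires projectiles.
; On BeginPlay it caches its parent actor as the owning pawn, or prints a debug string and destroys itself if that parent is not a pawn.
; Attack spawns the configured projectile class at the rifle's location and rotation, with the pawn's controller as owner and the pawn as instigator.
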(event EventBeginPlay
  (|CallParentFunction)
  (bind _aspawn (Utilities|Casting|CastToPawn (Actor|GetParentActor))
    (:then
      (Variables|Default|SetParent%20Pawn _aspawn))
    (:CastFailed
      (Development|PrintString "Bitch")
      (Actor|DestroyActor))))

(fn ConstructionScript)

(fn Attack
  (bind _parent_pawn (Variables|Default|GetParent%20Pawn))
  (Game|SpawnActorfromClass (Variables|Default|GetProjectile%20Class) (Math|Transform|MakeTransform (+ (Transformation|GetActorLocation) "0.000000,0.000000,0.000000") (Transformation|GetActorRotation) "1.000000,1.000000,1.000000") "Undefined" "MultiplyWithRoot" (Pawn|GetController _parent_pawn) _parent_pawn))